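; BP_RunnableWall is a wall actor that lets an overlapping BP_CharacterBase wall run.
; Tick, gated by DoOnce nodes, sweeps the cached player toward the wall mesh using a debug-drawn component trace, then sets Flying movement if they are moving, falling and holding only A or D.
; A delayed, self-resetting check restores Walking and flags landing when both keys are released.
; End overlap is empty, so the player reference is never cleared.
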(event Collision|EventActorBeginOverlap
  (params (OtherActor :type Actor%20Object%20Reference))
  (bind _asbp_character_base (Utilities|Casting|CastToBP_CharacterBase OtherActor))
  (Variables|Default|Setplayer%20cast _asbp_character_base))

(event Collision|EventActorEndOverlap
  (params (OtherActor :type Actor%20Object%20Reference)))

(event EventTick
  (params (DeltaSeconds :type Float%20%28single-precision%29))
  (bind _returnvalue (Game|GetPlayerController 0))
  (bind _player_cast (Variables|Default|Getplayer%20cast))
  (bind _player_cast_2 (Variables|Default|Getplayer%20cast))
  (bind _returnvalue_2 (Game|Player|IsInputKeyDown _returnvalue "A"))
  (bind _returnvalue_3 (Game|Player|IsInputKeyDown _returnvalue "D"))
  (bind _charactermovement (Variables|/Script/Engine.Character|GetCharacterMovement _player_cast))
  (Utilities|IsValid (Variables|Default|Getplayer%20cast)
    (:Is%20Valid
      (Utilities|FlowControl|Sequence
        (:then_0
          (Utilities|FlowControl|DoOnce false :!label _label
            (:Completed
              (Utilities|FlowControl|Sequence
                (:then_0
                  (bind _outhit (Collision|LineTraceComponent (Variables|Default|GetwallMesh) (Transformation|GetWorldLocation (Variables|/Script/Engine.Character|GetCapsuleComponent (Variables|Default|Getplayer%20cast))) (Transformation|GetWorldLocation (Variables|Default|GetwallMesh)) true true true))
                  (Transformation|SetActorRelativeLocation (Variables|Default|Getplayer%20cast) (.traceend _outhit) true))
                (:then_1
                  (if (Math|Boolean|ANDBoolean (> (Math|Vector|VectorLength (Transformation|GetVelocity (Variables|Default|Getplayer%20cast))) 0.0) (or (and _returnvalue_2 (not _returnvalue_3)) (and _returnvalue_3 (not _returnvalue_2))) (AI|Components|NavMovement|IsFalling (Variables|/Script/Engine.Character|GetCharacterMovement _player_cast_2)))
                    (Pawn|Components|CharacterMovement|SetMovementMode _charactermovement "MOVE_Flying" 0)
                    (Variables|/Game/FPS_Game/Blueprints/BP_CharacterBase.BP_CharacterBase_C|SetisWallRunning _player_cast true)
                    (else
                      (goto _label))))))))
        (:then_1
          (Utilities|FlowControl|DoOnce false :!label _label_2
            (:Completed
              (if (Variables|/Game/FPS_Game/Blueprints/BP_CharacterBase.BP_CharacterBase_C|GetisWallRunning _player_cast_2)
                (if (or (Game|Player|IsInputKeyDown (Game|GetPlayerController 0) "A") (Game|Player|IsInputKeyDown (Game|GetPlayerController 0) "D"))
                  (Utilities|FlowControl|RetriggerableDelay 0.5)
                  (goto _label_2 Reset)
                  (else
                    (Pawn|Components|CharacterMovement|SetMovementMode _charactermovement "MOVE_Walking" 0)
                    (Variables|/Game/FPS_Game/Blueprints/BP_CharacterBase.BP_CharacterBase_C|SetisWallRunning _player_cast false)
                    (Variables|/Game/FPS_Game/Blueprints/BP_CharacterBase.BP_CharacterBase_C|SethasLanded _player_cast true)
                    (Utilities|FlowControl|RetriggerableDelay 0.5)
                    (goto _label_2 Reset)))
                (else
                  (Utilities|FlowControl|Delay 0.2)
                  (goto _label_2 Reset))))))))))

(fn ConstructionScript)